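; Economy system Blueprint that exposes per-material resource data and signals resource count changes to the UI.
; Two lookup functions linearly search the Materials array by MaterialType, returning either the Count or, for GetMaterialTexture, the Mesh field.
; The AddResource event only calls CallUpdateUIResourceCount; this graph does not modify any counts itself.
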(event `/Game/Student/Blueprints/Interfaces/EconomyControl.AddResource`
  (params (`Adding?` :type Boolean) (Material :type "/Game/Student/Blueprints/Enums/Materials Enum" :default "NewEnumerator0"))
  (`self.UpdateUIResourceCount`))

(fn `GetMaterialCount`
  (params (Material :type "/Game/Student/Blueprints/Enums/Materials Enum" :default "NewEnumerator0"))
  (returns (Count :type Integer))
  (for _array_element (`self.Materials`)
    (bind (_materialtype _count) (break `/Game/Student/Blueprints/Enums/MaterialProperties` _array_element))
    (if (`|EnumEquality` _materialtype Material)
      (return _count))))

(fn `GetMaterialTexture`
  (params (Material :type "/Game/Student/Blueprints/Enums/Materials Enum" :default "NewEnumerator0"))
  (returns (Texture :type "Texture Object Reference"))
  (for _array_element (`self.Materials`)
    (bind (_materialtype _count _mesh) (break `/Game/Student/Blueprints/Enums/MaterialProperties` _array_element))
    (if (`|EnumEquality` Material _materialtype)
      (return _mesh))))

(fn `UserConstructionScript`)