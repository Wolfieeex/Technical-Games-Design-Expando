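; A resource button widget that starts and ends drag-and-drop of its assigned resource type.
; On press it gets the resource's texture through the game mode and attaches it to the resource widget as a drag image.
; On release it clears that image and sends the resource type to the widget as a drop.
; Hovering starts a two-second Help timer, cancelled on unhover, but Help only fetches the widget so far.
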(event `/Game/Student/Blueprints/Interfaces/ButtonControl.Construct`
  (add `self.OnPressed` (delegate `OnPressedEvent`))
  (add `self.OnReleased` (delegate `OnReleasedEvent`))
  (add `self.OnHovered` (delegate `OnHoveredEvent`))
  (add `self.OnUnhovered` (delegate `OnUnhoveredEvent`)))

(event `OnPressedEvent`
  (bind _returnvalue (`GameplayStatics.GetGameMode`))
  (bind _texture (message `/Game/Student/Blueprints/Interfaces/EconomyControl.GetMaterialTexture` _returnvalue (`self.ResourceType`)))
  (bind _ui (message `/Game/Student/Blueprints/Interfaces/ButtonControl.GetResourceWidget` _returnvalue))
  (`/Game/Student/Blueprints/User_Interface/Resource_OnScreen.AttachDragTexture` _ui _texture true))

(event `OnReleasedEvent`
  (bind _ui (message `/Game/Student/Blueprints/Interfaces/ButtonControl.GetResourceWidget` (`GameplayStatics.GetGameMode`)))
  (`/Game/Student/Blueprints/User_Interface/Resource_OnScreen.AttachDragTexture` _ui "/Game/ShutterstockImages/Resources/AlluminiumAlloy_Resource.AlluminiumAlloy_Resource" false)
  (message `/Game/Student/Blueprints/Interfaces/ButtonControl.DropDragButton` _ui (`self.ResourceType`)))

(event `OnHoveredEvent`
  (bind _returnvalue (`KismetSystemLibrary.K2_SetTimerDelegate` (delegate `Help`) 2.0)))

(event `OnUnhoveredEvent`
  (`KismetSystemLibrary.K2_ClearAndInvalidateTimerHandle` (stale `OnHoveredEvent` _returnvalue)))

(event `Help`
  (message `/Game/Student/Blueprints/Interfaces/ButtonControl.GetResourceWidget` (`GameplayStatics.GetGameMode`)))

(fn `GetMaterialCount`
  (params (Material :type "/Game/Student/Blueprints/Enums/Materials Enum" :default "NewEnumerator0"))
  (returns (Count :type Integer))
  (return 0))

(fn `GetMaterialTexture`
  (params (Material :type "/Game/Student/Blueprints/Enums/Materials Enum" :default "NewEnumerator0"))
  (returns (Texture :type "Texture Object Reference"))
  (return null))

(fn `GetResourceWidget`
  (returns (UI :type "/Game/Student/Blueprints/User_Interface/Resource_OnScreen Object Reference"))
  (return null))

(fn `PassResourceWidget`
  (params (UI :type "/Game/Student/Blueprints/User_Interface/Resource_OnScreen Object Reference"))
  (return))