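; Inventory button that shows a description on hover and toggles player UI when clicked.
; On Construct it binds its own hover, unhover and click events, with hover and unhover setting the visibility of the description image and text.
; A click fetches the resource widget through the game mode and calls PlayerUIToggle with the button's Type.
; GetResourceWidget and PassResourceWidget are empty here.
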(event `OnUnhoveredEvent`
  (`self.SetVisibility` (`self.DescriptionImage`) "Hidden")
  (`self.SetVisibility` (`self.DescriptionText`) "Hidden"))

(event `/Game/Student/Blueprints/Interfaces/ButtonControl.Construct`
  (add `self.OnHovered` (delegate `OnHoveredEvent`))
  (add `self.OnUnhovered` (delegate `OnUnhoveredEvent`))
  (add `self.OnClicked` (delegate `OnClickedEvent`)))

(event `OnClickedEvent`
  (bind _ui (message `/Game/Student/Blueprints/Interfaces/ButtonControl.GetResourceWidget` (`GameplayStatics.GetGameMode`)))
  (`/Game/Student/Blueprints/User_Interface/Resource_OnScreen.PlayerUIToggle` _ui (`self.Type`)))

(event `OnHoveredEvent`
  (`self.SetVisibility` (`self.DescriptionImage`) "Visible")
  (`self.SetVisibility` (`self.DescriptionText`) "Visible"))

(fn `GetResourceWidget`
  (returns (UI :type "/Game/Student/Blueprints/User_Interface/Resource_OnScreen Object Reference"))
  (return null))

(fn `PassResourceWidget`
  (params (UI :type "/Game/Student/Blueprints/User_Interface/Resource_OnScreen Object Reference"))
  (return))