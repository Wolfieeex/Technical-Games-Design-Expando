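; Grid manager Blueprint that sets up occupancy storage for a square tile grid when play begins.
; BeginPlay calls InitiateTiles, which resizes OccupationArray to MapSize squared, then walks the grid with nested column and row loops.
; The loops only store the current column and row indices; no tiles are spawned and no occupancy values are written.
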(event `self.ReceiveBeginPlay`
  (`self.Initiate_Tiles`))

(fn `Initiate_Tiles`
  (locals (CurrentCollumn :type Integer) (CurrentRow :type Integer))
  (bind _mapsize (`self.MapSize`))
  (`KismetArrayLibrary.Array_Resize` (`self.OccupationArray`) (* _mapsize _mapsize))
  (for _index (range (`self.MapSize`))
    (set `local.CurrentCollumn` _index)
    (for _index_2 (range (`self.MapSize`))
      (set `local.CurrentRow` _index_2))))

(fn `UserConstructionScript`)