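; Player controller for click or touch movement, providing helper functions to steer the controlled pawn toward a point in the world.
; Cursor and first-finger lookups return the hit location of a complex Visibility trace.
; A given location can drive either a SimpleMoveToLocation order with a cursor FX spawned at the target, or direct movement input toward it for follow-style steering.
; The file contains no input events calling these functions.
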(fn `FollowMouseOrFinger`
  (params (Location :type "Vector Structure"))
  (bind _returnvalue (`self.K2_GetPawn`))
  (`Pawn.AddMovementInput` _returnvalue (`KismetMathLibrary.GetDirectionUnitVector` (`self.K2_GetActorLocation` _returnvalue) Location) 1.0 false))

(fn `GetLocationUnderCursor`
  (returns (Location :type "Vector Structure"))
  (return (`.Location` (`GameplayStatics.BreakHitResult` (`self.GetHitResultUnderCursorByChannel` "TraceTypeQuery1")))))

(fn `GetLocationUnderFinger`
  (returns (Location :type "Vector Structure"))
  (return (`.Location` (`GameplayStatics.BreakHitResult` (`self.GetHitResultUnderFingerByChannel` "Touch1" "TraceTypeQuery1")))))

(fn `MoveToHitLocation`
  (params (Location :type "Vector Structure"))
  (`AIBlueprintHelperLibrary.SimpleMoveToLocation` self Location)
  (`NiagaraFunctionLibrary.SpawnSystemAtLocation` (`self.FXCursor`) Location))

(fn `UserConstructionScript`)