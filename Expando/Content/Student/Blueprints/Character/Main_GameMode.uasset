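; Game mode that owns the map grid and economy systems, acting as the central access point for both.
; On BeginPlay it spawns Grid_Manager, passes it the map settings to initialise tiles, then spawns EconomySystem.
; It forwards space reservations to the grid, exposes tile and occupancy arrays, and relays material textures from the economy.
; It also stores the resource widget passed to it; GetMaterialCount is a stub returning zero.
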(event `/Game/Student/Blueprints/Interfaces/ButtonControl.PassResourceWidget`
  (params (UI :type "/Game/Student/Blueprints/User_Interface/Resource_OnScreen Object Reference"))
  (set `self.MainMenu` UI))

(event `self.ReceiveBeginPlay`
  (bind _returnvalue (`|SpawnActorFromClass` "/Game/Student/Blueprints/Grid/Grid_Manager.Grid_Manager_C" (`KismetMathLibrary.MakeTransform` (0.0 0.0 0.0)) "AlwaysSpawn" "OverrideRootScale" null null))
  (bind _output_get (set `self.Grid_Manager` _returnvalue))
  (set `/Game/Student/Blueprints/Grid/Grid_Manager.MapSize` (`self.MapSize`) _output_get)
  (set `/Game/Student/Blueprints/Grid/Grid_Manager.GridSizeInUnits` (`self.GridUnits`) _output_get)
  (`/Game/Student/Blueprints/Grid/Grid_Manager.Initiate_Tiles` _output_get)
  (bind _returnvalue_2 (`|SpawnActorFromClass` "/Game/Student/Blueprints/Economy/EconomySystem.EconomySystem_C" (`KismetMathLibrary.MakeTransform` (0.0 0.0 0.0)) "AlwaysSpawn" "OverrideRootScale" null null))
  (set `self.EconomyManager` _returnvalue_2))

(event `/Game/Student/Blueprints/Interfaces/GridManager_Access.ReserveSpace`
  (params (CenterX :type Integer) (CenterY :type Integer) (Width :type Integer) (Length :type Integer))
  (`/Game/Student/Blueprints/Grid/Grid_Manager.Occupy Spaces` (`self.Grid_Manager`) CenterY CenterX Width Length))

(fn `GetGridManager`
  (returns (GridManager :type "/Game/Student/Blueprints/Grid/Grid_Manager Object Reference"))
  (return (`self.Grid_Manager`)))

(fn `GetMapProperties`
  (returns (MapSize :type Integer) (MapGridSize :type "Float (double-precision)"))
  (return (`self.MapSize`) (`self.GridUnits`)))

(fn `GetMaterialCount`
  (params (Material :type "/Game/Student/Blueprints/Enums/Materials Enum" :default "NewEnumerator0"))
  (returns (Count :type Integer))
  (return 0))

(fn `GetMaterialTexture`
  (params (Material :type "/Game/Student/Blueprints/Enums/Materials Enum" :default "NewEnumerator0"))
  (returns (Texture :type "Texture Object Reference"))
  (bind _texture (`/Game/Student/Blueprints/Interfaces/EconomyControl.GetMaterialTexture` (`self.EconomyManager`) Material))
  (return _texture))

(fn `GetOccupancyArray`
  (returns (OccupancyArray :type "Array of Boolean"))
  (return (`/Game/Student/Blueprints/Grid/Grid_Manager.OccupationArray` (`self.Grid_Manager`))))

(fn `GetResourceWidget`
  (returns (UI :type "/Game/Student/Blueprints/User_Interface/Resource_OnScreen Object Reference"))
  (return (`self.MainMenu`)))

(fn `GetTileArray`
  (returns (TileArray :type "Array of /Game/Student/Blueprints/Grid/Grid_Tile Object Reference"))
  (return (`/Game/Student/Blueprints/Grid/Grid_Manager.GridArray` (`self.Grid_Manager`))))

(fn `UserConstructionScript`)