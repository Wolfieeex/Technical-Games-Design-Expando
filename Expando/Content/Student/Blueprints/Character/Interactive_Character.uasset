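; Player character with movement, FOV zoom, resource UI toggles and a grid-based build mode for a small workshop.
; In build mode, Tick traces the cursor, snaps a rotatable ghost mesh to the grid and tints it by placement validity.
; Validity checks the data-table footprint against map bounds, occupancy and the character's position.
; Clicking adds the construction mesh through the GameMode's grid manager and reserves its tiles.
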(event `InputAction|LeftMouseClick`
  (params (Key :type "Key Structure"))
  (bind (_row _collumn) (`self.GetGridRowAndCollumnBasedOnWorldLocation` (`self.CurrentCursorLocation`)))
  (bind (_row_2 _collumn_2) (`self.GetGridRowAndCollumnBasedOnWorldLocation` (`self.CurrentCursorLocation`)))
  (bind (_row_3 _collumn_3) (`self.GetGridRowAndCollumnBasedOnWorldLocation` (`self.CurrentCursorLocation`)))
  (bind (_x _y) (`self.Calculate Location On Grid` _row _collumn))
  (:`Pressed`
    (if (`|EnumEquality` (`self.CurrentMode`) "NewEnumerator2")
      (if (`self.ConstructionPermission`)
        (bind _gridmanager (message `/Game/Student/Blueprints/Interfaces/GridManager_Access.GetGridManager` (`GameplayStatics.GetGameMode`)))
        (bind _returnvalue (`AddComponent|NODE_AddStaticMeshComponent-1` :`self` _gridmanager :`RelativeTransform` (`KismetMathLibrary.MakeTransform` (`KismetMathLibrary.MakeVector` _x _y 50.0) (`SceneComponent.K2_GetComponentRotation` (`self.ConstructionMesh`)))))
        (`StaticMeshComponent.SetStaticMesh` _returnvalue "/Game/Student/3DsMaxMesh/Constructions/Workshop_Small_Construction.Workshop_Small_Construction")
        (bind _returnvalue_2 (`|GetDataTableRow` "/Game/Student/Blueprints/Enums/BuildingConstructionDataTable.BuildingConstructionDataTable" "WkS")
          (:`then`
            (if (== (mod (`self.RotationAlteration`) 2) 0)
              (bind _returnvalue_3 (`|GetDataTableRow` "/Game/Student/Blueprints/Enums/BuildingConstructionDataTable.BuildingConstructionDataTable" "WkS")
                (:`then`
                  (message `/Game/Student/Blueprints/Interfaces/GridManager_Access.ReserveSpace` (`GameplayStatics.GetGameMode`) _collumn_3 _row_3 (`.Length_28_96879A7D4859D9A6214E438DF8E06A66` (break `/Game/Student/Blueprints/Enums/Structure_Data` _returnvalue_3)) (`.Width_27_0BE8360F4A0AF63BAEB0A0A43E14EBE5` (break `/Game/Student/Blueprints/Enums/Structure_Data` _returnvalue_3)))))
              (else
                (message `/Game/Student/Blueprints/Interfaces/GridManager_Access.ReserveSpace` (`GameplayStatics.GetGameMode`) _collumn_2 _row_2 (`.Width_27_0BE8360F4A0AF63BAEB0A0A43E14EBE5` (break `/Game/Student/Blueprints/Enums/Structure_Data` _returnvalue_2)) (`.Length_28_96879A7D4859D9A6214E438DF8E06A66` (break `/Game/Student/Blueprints/Enums/Structure_Data` _returnvalue_2)))))
            (`GameplayStatics.SpawnSound2D` "/Game/InternetAssets/SoundEffects/ConstructionStarted.ConstructionStarted" 1.0 1.0 0.0 null)
            (`self.ConstructionPlaced`)))
        (else
          (`GameplayStatics.SpawnSound2D` "/Game/InternetAssets/SoundEffects/Denial.Denial" 1.0 1.0 0.0 null))))))

(event `ContructionBlueprintRotated`
  (bind _allowed (`self.CheckContructionPermission` :!label _label))
  (set `self.ConstructionPermission` _allowed)
  (for _index (range 11)
    (`PrimitiveComponent.SetMaterial` (`self.ConstructionMesh`) _index (select `bool` (`self.ConstructionPermission`) :`false` (`self.OccupyMaterial`) :`true` (`self.FreeMaterial`)))))

(event `ConstructionPlaced`
  (goto _label))

(event `self.ReceiveTick`
  (params (DeltaSeconds :type "Float (single-precision)"))
  (bind (_row _collumn) (`self.GetGridRowAndCollumnBasedOnWorldLocation` (`self.CurrentCursorLocation`)))
  (bind (_worldlocation _worlddirection) (`PlayerController.DeprojectMousePositionToWorld` (`GameplayStatics.GetPlayerController` 0)))
  (bind (_row_2 _collumn_2) (`self.GetGridRowAndCollumnBasedOnWorldLocation` (`self.CurrentCursorLocation`)))
  (if (`|EnumEquality` (`self.CurrentMode`) "NewEnumerator2")
    (bind _outhit (`KismetSystemLibrary.LineTraceSingle` _worldlocation (+ _worldlocation (* _worlddirection 10000.0)) "TraceTypeQuery3"))
    (bind (_mapsize _mapgridsize) (message `/Game/Student/Blueprints/Interfaces/GridManager_Access.GetMapProperties` (`GameplayStatics.GetGameMode`)))
    (set `self.Map Size` _mapsize)
    (set `self.GridSizeInUnits` _mapgridsize)
    (bind (_bblockinghit _binitialoverlap _time _distance _location) (`GameplayStatics.BreakHitResult` _outhit))
    (set `self.CurrentCursorLocation` _location)
    (bind (_row_3 _collumn_3) (`self.GetGridRowAndCollumnBasedOnWorldLocation` _location))
    (bind (_x _y) (`self.Calculate Location On Grid` _row_3 _collumn_3))
    (`SceneComponent.K2_SetWorldLocation` (`self.ConstructionMesh`) (`KismetMathLibrary.MakeVector` _x _y) false false)
    (if (or (!= (`self.PreviousRowChecked`) _row) (!= _collumn (`self.PreviousCollumnChecked`)) (!= (`self.PreviousCharacterLocationCheck`) (`self.K2_GetActorLocation`) :`ErrorTolerance` 0.1))
      (set `self.PreviousCharacterLocationCheck` (`self.K2_GetActorLocation`))
      (set `self.PreviousRowChecked` _row_2)
      (set `self.PreviousCollumnChecked` _collumn_2)
      (goto _label))))

(event `InputAction|TestInteraction`
  (params (Key :type "Key Structure"))
  (bind _returnvalue (`GameplayStatics.GetPlayerController` 0))
  (:`Pressed`
    (`/Engine/EditorBlueprintResources/StandardMacros.FlipFlop`
      (:`A`
        (set `PlayerController.bShowMouseCursor` true _returnvalue)
        (set `self.CurrentMode` "NewEnumerator2")
        (`/Engine/EditorBlueprintResources/StandardMacros.DoOnce` false
          (:`Completed`
            (bind _gridmanager (message `/Game/Student/Blueprints/Interfaces/GridManager_Access.GetGridManager` (`GameplayStatics.GetGameMode`)))
            (bind _returnvalue_2 (`AddComponent|NODE_AddStaticMeshComponent-0` :`self` _gridmanager))
            (`StaticMeshComponent.SetStaticMesh` _returnvalue_2 "/Game/Student/3DsMaxMesh/Constructions/Workshop_Small_Ghost.Workshop_Small_Ghost")
            (bind _output_get (set `self.ConstructionMesh` _returnvalue_2))
            (`SceneComponent.SetVisibility` _output_get true false)
            (`PrimitiveComponent.SetCollisionEnabled` _output_get "NoCollision"))))
      (:`B`
        (set `PlayerController.bShowMouseCursor` false _returnvalue)
        (set `self.CurrentMode` "NewEnumerator0")
        (`SceneComponent.SetVisibility` (`self.ConstructionMesh`) false false)))))

(event `InputAction|Rotate`
  (params (Key :type "Key Structure"))
  (:`Pressed`
    (if (`|EnumEquality` (`self.CurrentMode`) "NewEnumerator2")
      (`self.ClampRotation`)
      (`SceneComponent.K2_AddWorldRotation` (`self.ConstructionMesh`) (struct :`Yaw` 90.0) false false)
      (`self.ContructionBlueprintRotated`))))

(event `self.ReceiveBeginPlay`
  (bind _returnvalue (`|CreateWidget` "/Game/Student/Blueprints/User_Interface/Resource_OnScreen.Resource_OnScreen_C"))
  (bind _output_get (set `self.MainUI` _returnvalue))
  (`UserWidget.AddToViewport` _output_get 0)
  (message `/Game/Student/Blueprints/Interfaces/ButtonControl.PassResourceWidget` (`GameplayStatics.GetGameMode`) _output_get))

(event `InputAxis|MoveUp`
  (params (AxisValue :type "Float (single-precision)"))
  ;[0 0.5605 1] Movement and Camera
  (`self.AddMovementInput` (`KismetMathLibrary.Vector_Forward`) AxisValue))

(event `InputAxis|MoveRight`
  (params (AxisValue :type "Float (single-precision)"))
  ;[0 0.5605 1] Movement and Camera
  (`self.AddMovementInput` (`KismetMathLibrary.Vector_Right`) AxisValue))

(event `InputAction|Inventory`
  (params (Key :type "Key Structure"))
  (:`Pressed`
    (`/Game/Student/Blueprints/User_Interface/Resource_OnScreen.PlayerUIToggle` (`self.MainUI`) "NewEnumerator0")))

(event `InputAction|Escape`
  (params (Key :type "Key Structure"))
  (:`Pressed`
    (`/Game/Student/Blueprints/User_Interface/Resource_OnScreen.PlayerUIToggle` (`self.MainUI`) "NewEnumerator2")))

(event `InputAction|ZoomIn`
  (params (Key :type "Key Structure"))
  ;[0 0.5605 1] Movement and Camera
  (:`Pressed`
    (`CameraComponent.SetFieldOfView` (`self.Camera`) (`KismetMathLibrary.FClamp` (+ (`CameraComponent.FieldOfView` (`self.Camera`)) -2.0) (`self.MinFieldOfView`) (`self.MaxFieldOfView`)))))

(event `InputAction|Resources`
  (params (Key :type "Key Structure"))
  (:`Pressed`
    (`/Game/Student/Blueprints/User_Interface/Resource_OnScreen.PlayerUIToggle` (`self.MainUI`) "NewEnumerator1")))

(event `InputAction|ZoomOut`
  (params (Key :type "Key Structure"))
  ;[0 0.5605 1] Movement and Camera
  (:`Pressed`
    (`CameraComponent.SetFieldOfView` (`self.Camera`) (`KismetMathLibrary.FClamp` (- (`CameraComponent.FieldOfView` (`self.Camera`)) -2.0) (`self.MinFieldOfView`) (`self.MaxFieldOfView`)))))

(fn `Calculate Location On Grid`
  (params (Row :type Integer) (Collumn :type Integer))
  (returns (X :type "Float (double-precision)") (Y :type "Float (double-precision)"))
  (bind _gridsizeinunits (`self.GridSizeInUnits`))
  (bind _returnvalue (/ _gridsizeinunits 2.0))
  (return (- (* (+ (/ (`self.Map Size`) -2) Row) _gridsizeinunits) _returnvalue) (- (* (+ (/ (`self.Map Size`) -2) Collumn) (`self.GridSizeInUnits`)) _returnvalue)))

(fn `CheckContructionPermission`
  (returns (Allowed :type Boolean))
  (locals (Width :type Integer) (Length :type Integer) (Occupancy :type "Array of Boolean") (Tiles :type "Array of /Game/Student/Blueprints/Grid/Grid_Tile Object Reference") (MinRowForCheck :type Integer) (MaxRowForCheck :type Integer) (MinCollumnForCheck :type Integer) (MaxCollumnForCheck :type Integer) (RowIndex :type Integer) (CollumnIndex :type Integer) (CharacterLocationForCheckOffset :type "Float (double-precision)" :default 100.0))
  (bind _returnvalue_x (`KismetMathLibrary.BreakVector` (`self.K2_GetActorLocation`)))
  (bind (_returnvalue_x_2 _returnvalue_y) (`KismetMathLibrary.BreakVector` (`self.K2_GetActorLocation`)))
  (bind _returnvalue_x_3 (`KismetMathLibrary.BreakVector` (`self.K2_GetActorLocation`)))
  (bind _returnvalue (`GameplayStatics.GetGameMode`))
  (bind (_returnvalue_x_4 _returnvalue_y_2) (`KismetMathLibrary.BreakVector` (`self.K2_GetActorLocation`)))
  (bind _characterlocationforcheckoffset (`local.CharacterLocationForCheckOffset`))
  (bind _characterlocationforcheckoffset_2 (`local.CharacterLocationForCheckOffset`))
  (bind _length (`local.Length`))
  (bind _width (`local.Width`))
  (bind _tilearray (message `/Game/Student/Blueprints/Interfaces/GridManager_Access.GetTileArray` _returnvalue))
  (set `local.Tiles` _tilearray)
  (bind _occupancyarray (message `/Game/Student/Blueprints/Interfaces/GridManager_Access.GetOccupancyArray` _returnvalue))
  (set `local.Occupancy` _occupancyarray)
  (bind _returnvalue_2 (`|GetDataTableRow` "/Game/Student/Blueprints/Enums/BuildingConstructionDataTable.BuildingConstructionDataTable" "WkS")
    (:`then`
      (if (== (mod (`self.RotationAlteration`) 2) 0)
        (bind (_name _width_2 _length_2) (break `/Game/Student/Blueprints/Enums/Structure_Data` _returnvalue_2))
        (set `local.Width` _length_2)
        (set `local.Length` _width_2)
        (else
          (set `local.Width` _width_2)
          (set `local.Length` _length_2)))
      (if (!= (mod (`local.Width`) 2) 0)
        (set `local.MinCollumnForCheck` (- (`self.PreviousCollumnChecked`) (/ (- (`local.Width`) 1) 2)))
        (set `local.MaxCollumnForCheck` (+ (`self.PreviousCollumnChecked`) (/ (- (`local.Width`) 1) 2)))
        (else
          (set `local.MinCollumnForCheck` (- (`self.PreviousCollumnChecked`) (- (/ (`local.Width`) 2) 1)))
          (set `local.MaxCollumnForCheck` (+ (`self.PreviousCollumnChecked`) (/ (`local.Width`) 2)))))
      (if (!= (mod (`local.Length`) 2) 0)
        (set `local.MinRowForCheck` (- (`self.PreviousRowChecked`) (/ (- (`local.Length`) 1) 2)))
        (set `local.MaxRowForCheck` (+ (`self.PreviousRowChecked`) (/ (- (`local.Length`) 1) 2)))
        (else
          (set `local.MinRowForCheck` (- (`self.PreviousRowChecked`) (- (/ (`local.Length`) 2) 1)))
          (set `local.MaxRowForCheck` (+ (`self.PreviousRowChecked`) (/ (`local.Length`) 2)))))
      (if (== (`local.Length`) 1)
        (set `local.MinRowForCheck` _length)
        (set `local.MaxRowForCheck` _length))
      (if (== (`local.Width`) 1)
        (set `local.MinCollumnForCheck` _width)
        (set `local.MaxCollumnForCheck` _width))
      (if (or (< (`local.MinRowForCheck`) 1) (< (`local.MinCollumnForCheck`) 1) (> (`local.MaxCollumnForCheck`) (`self.Map Size`)) (> (`local.MaxRowForCheck`) (`self.Map Size`)))
        (return false)
        (else
          (for _index (range (`local.MinRowForCheck`) (+ (`local.MaxRowForCheck`) 1))
            (set `local.RowIndex` _index)
            (for _index_2 (range (`local.MinCollumnForCheck`) (+ (`local.MaxCollumnForCheck`) 1))
              (set `local.CollumnIndex` _index_2)
              (if (`|GetArrayItem` (`local.Occupancy`) (+ (`local.RowIndex`) (* (- (`local.CollumnIndex`) 1) (`self.Map Size`))))
                (return false))))
          (return (not (and (> _returnvalue_y_2 (- (`.Y` (`self.Calculate Location On Grid` (`local.MinRowForCheck`) (`local.MinCollumnForCheck`))) _characterlocationforcheckoffset_2)) (< _returnvalue_y (+ (`.Y` (`self.Calculate Location On Grid` (`local.MaxRowForCheck`) (`local.MaxCollumnForCheck`))) _characterlocationforcheckoffset_2)) (> _returnvalue_x_3 (- (`self.Calculate Location On Grid` (`local.MinRowForCheck`) (`local.MinCollumnForCheck`)) _characterlocationforcheckoffset)) (< _returnvalue_x (+ (`self.Calculate Location On Grid` (`local.MaxRowForCheck`) (`local.MaxCollumnForCheck`)) _characterlocationforcheckoffset))))))))))

(fn `ClampRotation`
  (bind _result (`/Engine/EditorBlueprintResources/StandardMacros.IncrementInt` (`self.RotationAlteration`))
    (:`  `
      (if (> _result 4)
        (set `self.RotationAlteration` 1)))))

(fn `GetGridManager`
  (returns (GridManager :type "/Game/Student/Blueprints/Grid/Grid_Manager Object Reference"))
  (return null))

(fn `GetGridRowAndCollumnBasedOnWorldLocation`
  (params (Location :type "Vector Structure"))
  (returns (Row :type Integer) (Collumn :type Integer))
  (bind (_x _y) (`KismetMathLibrary.BreakVector3f` Location))
  (bind _gridsizeinunits (`self.GridSizeInUnits`))
  (return (+ (/ (`self.Map Size`) 2) (`KismetMathLibrary.Round` (/ (+ (/ (`self.GridSizeInUnits`) 2.0) _x) _gridsizeinunits))) (+ (`KismetMathLibrary.Round` (/ (+ _y (/ (`self.GridSizeInUnits`) 2.0)) _gridsizeinunits)) (/ (`self.Map Size`) 2))))

(fn `GetMapProperties`
  (returns (MapSize :type Integer) (MapGridSize :type "Float (double-precision)"))
  (return 0 0.0))

(fn `GetOccupancyArray`
  (returns (OccupancyArray :type "Array of Boolean"))
  (return))

(fn `GetResourceWidget`
  (returns (UI :type "/Game/Student/Blueprints/User_Interface/Resource_OnScreen Object Reference"))
  (return null))

(fn `GetTileArray`
  (returns (TileArray :type "Array of /Game/Student/Blueprints/Grid/Grid_Tile Object Reference"))
  (return))

(fn `UserConstructionScript`
  (bind _returnvalue (`KismetMaterialLibrary.CreateDynamicMaterialInstance` "/Game/Student/Materials/ConstructionMode/SpaceCanBuild.SpaceCanBuild"))
  (set `self.FreeMaterial` _returnvalue)
  (bind _returnvalue_2 (`KismetMaterialLibrary.CreateDynamicMaterialInstance` "/Game/Student/Materials/ConstructionMode/SpaceSignicate.SpaceSignicate"))
  (set `self.OccupyMaterial` _returnvalue_2))